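; BP_Actor1 is an actor with no clear gameplay purpose, apparently a scratch or test Blueprint.
; On BeginPlay it calls GetAllActorsOfClass without using the result, then runs three short chained Delays with nothing after them.
; Unreachable fragments hold unrelated nodes such as player creation, AI spawning and movement, actor destruction and an editor cast.
; Overlap and Tick are disabled, and the construction script is empty.
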(event `self.ReceiveBeginPlay`
  (`GameplayStatics.GetAllActorsOfClass` null)
  (`KismetSystemLibrary.Delay` 0.2)
  (`KismetSystemLibrary.Delay` 0.2)
  (`KismetSystemLibrary.Delay` 0.2))

(fn `UserConstructionScript`)